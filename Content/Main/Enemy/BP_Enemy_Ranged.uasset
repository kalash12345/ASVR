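; Ranged enemy character that spawns a rifle on BeginPlay, attaches it to a hand-weapon socket on its mesh and reports it equipped.
; Attack plays a firing montage whose notify traces from the weapon to the AI controller's AttackTarget, sending fixed damage only when nothing blocks visibility.
; Montage completion or interruption signals attack end.
; It also defines per-state walk speeds and ideal attack and defend ranges.
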(event Custom|Shoot
  ;[0.003922 0.003922 0.003922] Attack Functionality
)

(event EventBeginPlay
  (|CallParentFunction)
  (CallFunction|EquipWeapon))

(event EventEquipWeapon
  ;[0.003922 0.003922 0.003922] Spawn Rifle
  (bind _returnvalue (Game|SpawnActorfromClass "/Game/Main/Weapons/BP_Weapon_Rifle.BP_Weapon_Rifle_C" (Math|Transform|MakeTransform "0, 0, 0") "Undefined" "MultiplyWithRoot" 0 0))
  (bind _output_get (Variables|Default|SetWeaponActor _returnvalue))
  (Transformation|AttachComponentToComponent _output_get (Variables|Character|GetMesh) "AK47Socket" "SnapToTarget" "SnapToTarget" "SnapToTarget" true)
  (Variables|Default|SetIsWieldingWeapon true)
  (Default|CallOnWeaponEquipped))

(event EventAttack
  ;[0.003922 0.003922 0.003922] Attack Functionality
  (bind _notifyname (Animation|Montage|PlayMontage (Variables|Character|GetMesh) "/Game/Main/Enemy/Anims/Ranged/Firing_Rifle_Montage.Firing_Rifle_Montage")
    (:OnCompleted
      (Default|CallOnAttackEnd :!label _label))
    (:OnInterrupted
      (goto _label))
    (:OnNotifyBegin
      (switch name _notifyname
        (:Fire
          (bind _asaic_enemy_base (Utilities|Casting|CastToAIC_EnemyBase (AI|GetAIController self)))
          (bind _attack_target (Variables|/Game/Main/Enemy/AI_Workflow/AIC_EnemyBase.AIC_EnemyBase_C|GetAttack%20Target _asaic_enemy_base)
            (:then
              (bind _returnvalue (Collision|LineTraceByChannel (Transformation|GetActorLocation (Variables|Default|GetWeaponActor)) (Transformation|GetActorLocation _attack_target) "TraceTypeQuery1" false 0 "None"))
              (if (not _returnvalue)
                (Class|BPIDamagable|TakeDamage(Message) _attack_target (Utilities|Struct|MakeS_DamageInfo 2e+01 "NewEnumerator2"))))
            (:else)))))))

(fn ConstructionScript
  (|CallParentFunction))

(fn SetMovementSpeed
  (params (Speed :type E_MovementSpeed%20Enum :default "NewEnumerator0"))
  (bind _output_get (Variables|/Script/Engine.CharacterMovementComponent|SetMaxWalkSpeed (Variables|Character|GetCharacterMovement) (Utilities|Select :Index Speed :NewEnumerator0 0.0 :NewEnumerator1 2e+02 :NewEnumerator2 3e+02 :NewEnumerator3 5e+02)))
  (return _output_get))

(fn GetIdealRange
  (return 8e+02 8e+02))
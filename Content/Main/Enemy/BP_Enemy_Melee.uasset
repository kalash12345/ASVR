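; BP_Enemy_Melee is a melee enemy that equips, swings and sheathes a machete, driven by montages.
; Montage notifies time the gameplay: spawning and socketing the weapon, destroying it on unequip, and firing a forward sphere trace that damages a pawn it hits.
; Attacks make the damage system uninterruptible until the montage completes or is interrupted.
; Dispatchers signal when attack, equip and unequip end.
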(event EventEquipWeapon
  ;[0.003922 0.003922 0.003922] Spawn Machete
  (bind _notifyname (Animation|Montage|PlayMontage (Variables|Character|GetMesh) "/Game/Main/Enemy/Anims/Melee/Unsheath_Sword_Montage.Unsheath_Sword_Montage")
    (:OnCompleted
      (Default|CallOnWeaponEquipped))
    (:OnNotifyBegin
      (switch name _notifyname
        (:Hold%20Machete
          (bind _returnvalue (Game|SpawnActorfromClass "/Game/Main/Weapons/BP_Weapon_Melee.BP_Weapon_Melee_C" (Transformation|GetActorTransform) "Undefined" "MultiplyWithRoot" 0 0))
          (bind _output_get (Variables|Default|SetWeaponActor _returnvalue))
          (Transformation|AttachComponentToComponent _output_get (Variables|Character|GetMesh) "MacheteSocket" "SnapToTarget" "SnapToTarget" "SnapToTarget" true)
          (Variables|Default|SetIsWieldingWeapon true))))))

(event EventUnequipWeapon
  ;[0.003922 0.003922 0.003922] Sheath Machete
  (bind _notifyname (Animation|Montage|PlayMontage (Variables|Character|GetMesh) "/Game/Main/Enemy/Anims/Melee/Sheathing_Sword_Montage.Sheathing_Sword_Montage")
    (:OnCompleted
      (Default|CallOnWeaponUnequipped))
    (:OnNotifyBegin
      (switch name _notifyname
        (:Drop%20Machete
          (Actor|DestroyActor (Variables|Default|GetWeaponActor))
          (Variables|Default|SetIsWieldingWeapon false))))))

(event EventBeginPlay
  (|CallParentFunction))

(event EventAttack
  (bind _returnvalue (Transformation|GetActorLocation))
  (bind _bpc_damagesystem (Variables|Default|GetBPC_DamageSystem))
  ;[0.003922 0.003922 0.003922] Attack Montage
  (bind _notifyname (Animation|Montage|PlayMontage (Variables|Character|GetMesh) "/Game/Main/Enemy/Anims/Melee/SwordSlash_Montage.SwordSlash_Montage")
    (:then
      (Variables|/Game/DamageSystem/BPC_DamageSystem.BPC_DamageSystem_C|SetIsInterruptible _bpc_damagesystem false))
    (:OnCompleted
      (Default|CallOnAttackEnd :!label _label)
      (Variables|/Game/DamageSystem/BPC_DamageSystem.BPC_DamageSystem_C|SetIsInterruptible _bpc_damagesystem true))
    (:OnInterrupted
      (goto _label))
    (:OnNotifyBegin
      (switch name _notifyname
        (:Slash
          (bind (_outhit _returnvalue_2) (Collision|SphereTraceForObjects _returnvalue (+ _returnvalue (* (Transformation|GetActorForwardVector) 3e+02)) 2e+01 (Utilities|Array|MakeArray "ObjectTypeQuery3") false 0 "None"))
          (if _returnvalue_2
            (Class|BPIDamagable|TakeDamage(Message) (.HitActor (Collision|BreakHitResult _outhit)) (Utilities|Struct|MakeS_DamageInfo 35.0 "NewEnumerator1"))))))))

(fn ConstructionScript
  (|CallParentFunction))
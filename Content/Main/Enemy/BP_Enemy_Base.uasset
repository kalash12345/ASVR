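; BP_Enemy_Base is the base enemy character, linking a damage component to an AIC_EnemyBase AI controller.
; On death it ragdolls the mesh, stops the AI brain and sets the Dead state.
; Hits halt movement, set Frozen and play a reaction montage, then resume attacking the last known target.
; Functions expose health, healing and damage via the component, plus patrol route, combat ranges and enum-based movement speed.
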(event Custom|OnDeath
  (bind _mesh (Variables|Character|GetMesh))
  ;[0.003922 0.003922 0.003922] Death Functionality
  (Physics|SetSimulatePhysics _mesh true)
  (Collision|SetCollisionEnabled _mesh "QueryAndPhysics")
  (AI|Logic|StopLogic (Variables|/Script/AIModule.AIController|GetBrainComponent (Variables|Default|GetAICEnemyBase)) "")
  (Default|SetStateasDead (Variables|Default|GetAICEnemyBase)))

(event Custom|HitResponse
  (params (DamageResponse :type E_DamageResponse%20Enum :default "NewEnumerator0"))
  (bind _aicenemybase (Variables|Default|GetAICEnemyBase))
  (Components|Movement|StopMovementImmediately (Variables|Character|GetCharacterMovement))
  (Default|SetStateasFrozen _aicenemybase)
  (Animation|Montage|PlayMontage (Variables|Character|GetMesh) (Variables|Default|GetHitReaction)
    (:OnCompleted
      _)
    (:OnInterrupted
      _))
  (Default|SetStateasAttacking _aicenemybase 0 true))

(event EventBeginPlay
  (bind _bpc_damagesystem (Variables|Default|GetBPC_DamageSystem))
  (bind _asaic_enemy_base (Utilities|Casting|CastToAIC_EnemyBase (AI|GetAIController self)))
  (Variables|Default|SetAICEnemyBase _asaic_enemy_base)
  (EventDispatchers|AssignOnDeath _bpc_damagesystem (EventDispatchers|CreateEvent :!event Custom|OnDeath))
  (EventDispatchers|AssignOnDamageResponse _bpc_damagesystem (EventDispatchers|CreateEvent :!event Custom|HitResponse)))

(fn ConstructionScript)

(fn GetCurrentHealth
  (return (Variables|/Game/DamageSystem/BPC_DamageSystem.BPC_DamageSystem_C|GetHealth (Variables|Default|GetBPC_DamageSystem))))

(fn GetIdealRange
  (return 1.5e+02 3.5e+02))

(fn GetMaxHealth
  (return (Variables|/Game/DamageSystem/BPC_DamageSystem.BPC_DamageSystem_C|GetMaxHealth (Variables|Default|GetBPC_DamageSystem))))

(fn GetPatrolRoute
  (return (Variables|AI|GetPatrolRoute)))

(fn Heal
  (params (Amount :type Float%20%28double-precision%29))
  (bind _newhealth (Default|Heal (Variables|Default|GetBPC_DamageSystem) Amount))
  (return _newhealth))

(fn IsDead
  (return (Variables|/Game/DamageSystem/BPC_DamageSystem.BPC_DamageSystem_C|GetIsDead (Variables|Default|GetBPC_DamageSystem))))

(fn SetMovementSpeed
  (params (Speed :type E_MovementSpeed%20Enum :default "NewEnumerator0"))
  (bind _output_get (Variables|/Script/Engine.CharacterMovementComponent|SetMaxWalkSpeed (Variables|Character|GetCharacterMovement) (Utilities|Select :Index Speed :NewEnumerator0 0.0 :NewEnumerator1 1e+02 :NewEnumerator2 3e+02 :NewEnumerator3 5e+02)))
  (return _output_get))

(fn TakeDamage
  (params (DamageInfo :type S%20Damage%20Info%20Structure))
  (bind _wasdamaged (Default|TakeDamage (Variables|Default|GetBPC_DamageSystem) DamageInfo))
  (return _wasdamaged))